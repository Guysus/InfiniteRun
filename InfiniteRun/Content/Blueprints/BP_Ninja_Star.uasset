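; BP_Ninja_Star is a ninja star hazard that sets a GameOver flag when its collision sphere overlaps the first player's character.
; On BeginPlay it assigns the A_NinjaStar flipbook and spawns another BP_Ninja_Star at a fixed offset from its root transform.
; Each spawned star repeats that spawn with no stop condition, forming a self-replicating chain.
; The GameOver event has no logic.
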(event `self.Sphere.OnComponentBeginOverlap`
  (params (OverlappedComponent :type "PrimitiveComponent Object Reference") (OtherActor :type "Actor Object Reference") (OtherComp :type "PrimitiveComponent Object Reference") (OtherBodyIndex :type Integer) (bFromSweep :type Boolean) (SweepResult :type "HitResult Structure (by ref)"))
  (if (== OtherActor (`GameplayStatics.GetPlayerCharacter` 0))
    (set `self.Game Over` true)))

(event `self.ReceiveBeginPlay`
  (bind (_returnvalue_location _returnvalue_rotation _returnvalue_scale) (`KismetMathLibrary.BreakTransform` (`SceneComponent.K2_GetComponentToWorld` (`self.DefaultSceneRoot`))))
  (`|SpawnActorFromClass` "BP_Ninja_Star_C" (`KismetMathLibrary.MakeTransform` (+ _returnvalue_location (-500.0 -10.0 300.0)) _returnvalue_rotation _returnvalue_scale) "AlwaysSpawn" "MultiplyWithRoot" null null)
  (`PaperFlipbookComponent.SetFlipbook` (`self.NinjaStar`) "/Game/Sprites/A_NinjaStar.A_NinjaStar"))

(event `GameOver`)

(fn `UserConstructionScript`)